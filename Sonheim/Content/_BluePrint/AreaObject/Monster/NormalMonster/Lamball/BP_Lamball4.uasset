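; Lamball monster variant that issues itself a resource voice command and supports switchable facial expressions.
; Three seconds after BeginPlay it sends a forced AIVoiceCommand with one of two random resource IDs.
; ChangeFace copies preset mouth and eye vectors into the Default parameter of MPC_Mouth and MPC_Eye; as these collections are global, materials reading them share the expression.
; Other command and nearby-resource lookup nodes are unconnected.
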(event `self.ReceiveBeginPlay`
  (`KismetSystemLibrary.Delay` 3.0)
  (`self.AIVoiceCommand` (* (`KismetMathLibrary.RandomIntegerInRange` 1 2) 5) true))

(event `self.ChangeFace`
  (params (Feel :type Integer))
  (switch `int` Feel
    (:`0`
      (bind _returnvalue (`KismetMaterialLibrary.GetVectorParameterValue` "/Game/_Resource/Monster/Lamball/MPC_Mouth.MPC_Mouth" "Smile"))
      (`KismetMaterialLibrary.SetVectorParameterValue` "/Game/_Resource/Monster/Lamball/MPC_Mouth.MPC_Mouth" "Default" _returnvalue)
      (bind _returnvalue_2 (`KismetMaterialLibrary.GetVectorParameterValue` "/Game/_Resource/Monster/Lamball/MPC_Eye.MPC_Eye" "Smile"))
      (`KismetMaterialLibrary.SetVectorParameterValue` "/Game/_Resource/Monster/Lamball/MPC_Eye.MPC_Eye" "Default" _returnvalue_2))
    (:`1`
      (bind _returnvalue_3 (`KismetMaterialLibrary.GetVectorParameterValue` "/Game/_Resource/Monster/Lamball/MPC_Mouth.MPC_Mouth" "Fun"))
      (`KismetMaterialLibrary.SetVectorParameterValue` "/Game/_Resource/Monster/Lamball/MPC_Mouth.MPC_Mouth" "Default" _returnvalue_3)
      (bind _returnvalue_4 (`KismetMaterialLibrary.GetVectorParameterValue` "/Game/_Resource/Monster/Lamball/MPC_Eye.MPC_Eye" "Fun"))
      (`KismetMaterialLibrary.SetVectorParameterValue` "/Game/_Resource/Monster/Lamball/MPC_Eye.MPC_Eye" "Default" _returnvalue_4))
    (:`2`
      (bind _returnvalue_5 (`KismetMaterialLibrary.GetVectorParameterValue` "/Game/_Resource/Monster/Lamball/MPC_Mouth.MPC_Mouth" "Ouch"))
      (`KismetMaterialLibrary.SetVectorParameterValue` "/Game/_Resource/Monster/Lamball/MPC_Mouth.MPC_Mouth" "Default" _returnvalue_5)
      (bind _returnvalue_6 (`KismetMaterialLibrary.GetVectorParameterValue` "/Game/_Resource/Monster/Lamball/MPC_Eye.MPC_Eye" "Die"))
      (`KismetMaterialLibrary.SetVectorParameterValue` "/Game/_Resource/Monster/Lamball/MPC_Eye.MPC_Eye" "Default" _returnvalue_6))
    (:`3`
      (bind _returnvalue_7 (`KismetMaterialLibrary.GetVectorParameterValue` "/Game/_Resource/Monster/Lamball/MPC_Mouth.MPC_Mouth" "Sad"))
      (`KismetMaterialLibrary.SetVectorParameterValue` "/Game/_Resource/Monster/Lamball/MPC_Mouth.MPC_Mouth" "Default" _returnvalue_7)
      (bind _returnvalue_8 (`KismetMaterialLibrary.GetVectorParameterValue` "/Game/_Resource/Monster/Lamball/MPC_Eye.MPC_Eye" "Sad"))
      (`KismetMaterialLibrary.SetVectorParameterValue` "/Game/_Resource/Monster/Lamball/MPC_Eye.MPC_Eye" "Default" _returnvalue_8))))

(fn `UserConstructionScript`)